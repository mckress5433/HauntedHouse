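; Gameplay ability that toggles the player's options phone, switching between UI and game input.
; Activation spawns the phone on authority via a helper that attaches it to the character's hand-held phone socket, then sets UI input and narrows camera FOV.
; Ending stops mesh animation and destroys the phone.
; For the local controller, it also restores game input, cancels camera interpolation and widens FOV back.
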(event Ability|EventActivateAbility
  (bind _asin_game_player_state_bp (Utilities|Casting|CastToInGamePlayerState_BP (Ability|GetOwningActorfromActorInfo)))
  (bind _asin_game_character_bp (Utilities|Casting|CastToInGameCharacter_BP (PlayerState|GetPawn _asin_game_player_state_bp)))
  (bind _output_get (Variables|Default|SetInGameCharacter _asin_game_character_bp))
  (Ability|HasAuthority
    (:True
      (|SpawnandAttachPhone _output_get))
    (:False
      _))
  (bind _asin_game_player_controller_bp (Utilities|Casting|CastToInGamePlayerController_BP (Pawn|GetController (Variables|Default|GetInGameCharacter))))
  (Class|InGamePlayerController|SetUIInputMode _asin_game_player_controller_bp)
  (bind _cameracomp (Variables|/Script/HauntedHouse.InGameCharacter|GetCameraComp (Variables|Default|GetInGameCharacter))
    (:then
      (Camera|SetFieldOfView _cameracomp 65.0))
    (:else)))

(event Ability|EventOnEndAbility
  (params (bWasCancelled :type Boolean))
  (bind _ingamecharacter (Variables|Default|GetInGameCharacter))
  (Audio|Components|Audio|Stop (Variables|/Script/Engine.Character|GetMesh (Variables|Default|GetInGameCharacter)))
  (bind _phonereference (Variables|Default|GetPhoneReference)
    (:then
      (Actor|DestroyActor _phonereference))
    (:else
      _))
  (bind _asin_game_player_controller_bp (Utilities|Casting|CastToInGamePlayerController_BP (Pawn|GetController _ingamecharacter)))
  (if (Pawn|IsLocalPlayerController _asin_game_player_controller_bp)
    (Class|InGamePlayerController|SetGameInputMode _asin_game_player_controller_bp)
    (Class|InGameCharacter|CancelCameraInterpolation _ingamecharacter)
    (bind _cameracomp (Variables|/Script/HauntedHouse.InGameCharacter|GetCameraComp _ingamecharacter)
      (:then
        (Camera|SetFieldOfView _cameracomp 9e+01))
      (:else))))