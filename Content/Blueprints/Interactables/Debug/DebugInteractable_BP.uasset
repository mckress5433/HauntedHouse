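; Debug interactable actor that visualizes the state of its Interactable component through the color of a cube.
; BeginPlay creates a dynamic material instance on the cube and sets it to red.
; Interaction progress, scaled from a percentage, lerps the color from red to green unless a one-time interaction has already triggered.
; On interact, the cube turns yellow if the component reports it has been triggered, otherwise red.
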(event OnUpdateInteractionProgressEvent(Interactable)
  (params (Progress :type Byte :default 0))
  (bind _interactable (Variables|Default|GetInteractable))
  (if (not (and (Class|InteractableComponent|GetHasBeenTriggered _interactable) (Class|InteractableComponent|GetOnlyInteractOnce _interactable)))
    (Rendering|Material|SetVectorParameterValue (Variables|Default|GetMaterialInstance) "Color" (Math|Color|Lerp(LinearColor) "(R=1.000000,G=0.000000,B=0.000000,A=1.000000)" "(R=0.000000,G=1.000000,B=0.031859,A=1.000000)" (/ (Math|Conversions|ToFloat(Byte) Progress) 1e+02)) :!class /Script/Engine.MaterialInstanceDynamic)))

(event OnInteractEvent(Interactable)
  (Rendering|Material|SetVectorParameterValue (Variables|Default|GetMaterialInstance) "Color" (select (Class|InteractableComponent|GetHasBeenTriggered (Variables|Default|GetInteractable)) "(R=1.000000,G=1.000000,B=0.000000,A=1.000000)" "(R=1.000000,G=0.000000,B=0.000000,A=1.000000)") :!class /Script/Engine.MaterialInstanceDynamic))

(event EventBeginPlay
  (bind _returnvalue (Rendering|Material|CreateDynamicMaterialInstance (Variables|Default|GetCube) 0 "/Engine/BasicShapes/BasicShapeMaterial.BasicShapeMaterial" "None" :!class /Script/Engine.PrimitiveComponent))
  (bind _output_get (Variables|Default|SetMaterialInstance _returnvalue))
  (bind _output_get_2 (Variables|Default|SetColor "(R=1.000000,G=0.000000,B=0.000000,A=1.000000)"))
  (Rendering|Material|SetVectorParameterValue _output_get "Color" _output_get_2 :!class /Script/Engine.MaterialInstanceDynamic))

(fn ConstructionScript)